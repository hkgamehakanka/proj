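; VertigoHKgameSave is a save-game style data container for remembered player login details and player data.
; One save/load function pair sets and returns the remember flag (Hatirla), name, password (Parola) and ID.
; A second pair does the same for PlayerBilgisi (player info), sharing that remember flag.
; The functions only copy variables, with no slot read/write, validation or encryption here.
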(fn LoadVertigoGames
  (return (Variables|Default|GetHatirla) (Variables|Default|GetVertigoName) (Variables|Default|GetVertigoParola) (Variables|Default|GetVertigoID)))

(fn SaveVertigoGames
  (params (Hatirla :type Boolean) (VertigoName :type String) (VertigoParola :type String) (VertigoID :type String))
  (Variables|Default|SetHatirla Hatirla)
  (Variables|Default|SetVertigoName VertigoName)
  (Variables|Default|SetVertigoParola VertigoParola)
  (Variables|Default|SetVertigoID VertigoID))

(fn LoadVertigoData
  (return (Variables|Default|GetHatirla) (Variables|Default|GetPlayerBilgisi)))

(fn SaveVertigoData
  (params (Hatirla :type Boolean) (VertigoData :type Player%20Bilgisi%20Structure))
  (Variables|Default|SetHatirla Hatirla)
  (Variables|Default|SetPlayerBilgisi VertigoData))