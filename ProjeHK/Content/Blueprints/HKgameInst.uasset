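; HKgameInst, apparently the game instance, switches the game's menu widgets through one MainMenu function.
; An enum selects the Exit, Lobby, Vertigo menu or Error widget, each created on first use and cached.
; Showing one adds it to the viewport with UI-only input and a visible cursor.
; OpenHK toggles only Exit and Lobby; Game and Error always open, and HataText is unused.
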(fn MainMenu
  (params (MenuEnum :type MenuEnumHK%20Enum :default "NewEnumerator0") (OpenHK :type Boolean) (HataText :type String))
  (bind _returnvalue (Game|GetPlayerController 0))
  (bind _returnvalue_2 (Game|GetPlayerController 0))
  (bind _returnvalue_3 (Game|GetPlayerController 0))
  (bind _returnvalue_4 (Game|GetPlayerController 0))
  (switch Utilities|FlowControl|Switch|SwitchonMenuEnumHK MenuEnum
    (:NewEnumerator0
      ;[1 0.2036 0 0.5] Create Exit Widget
      (bind _exitwgt (Variables|Default|GetExitWgt)
        (:then
          _)
        (:else
          (bind _returnvalue_5 (UserInterface|CreateWidget "/Game/Widget/Exit.Exit_C" _returnvalue))
          (Variables|Default|SetExitWgt _returnvalue_5)))
      (if OpenHK
        (UserInterface|Viewport|AddtoViewport _exitwgt 1)
        (Input|SetInputModeUIOnly _returnvalue _exitwgt "DoNotLock")
        (Variables|/Script/Engine.PlayerController|SetbShowMouseCursor _returnvalue true)
        (else
          (Widget|RemovefromParent _exitwgt))))
    (:NewEnumerator2
      ;[1 0.2036 0 0.5] Create Loby Widget
      (bind _lobywgt (Variables|Default|GetLobyWgt)
        (:then
          _)
        (:else
          (bind _returnvalue_6 (UserInterface|CreateWidget "/Game/Widget/LobiWgt.LobiWgt_C" _returnvalue_4))
          (Variables|Default|SetLobyWgt _returnvalue_6)))
      (if OpenHK
        (UserInterface|Viewport|AddtoViewport _lobywgt 1)
        (Input|SetInputModeUIOnly _returnvalue_4 _lobywgt "DoNotLock")
        (Variables|/Script/Engine.PlayerController|SetbShowMouseCursor _returnvalue_4 true)
        (else
          (Widget|RemovefromParent _lobywgt))))
    (:NewEnumerator3
      ;[1 0.2036 0 0.5] Create Login Widget
      (bind _vertigowgt (Variables|Default|GetVertigoWgt)
        (:then
          _)
        (:else
          (bind _returnvalue_7 (UserInterface|CreateWidget "/Game/Widget/VertigoMenu.VertigoMenu_C" _returnvalue_2))
          (Variables|Default|SetVertigoWgt _returnvalue_7)))
      (if true
        (UserInterface|Viewport|AddtoViewport _vertigowgt 1)
        (Input|SetInputModeUIOnly _returnvalue_2 _vertigowgt "DoNotLock")
        (Variables|/Script/Engine.PlayerController|SetbShowMouseCursor _returnvalue_2 true)
        (else
          (Widget|RemovefromParent _vertigowgt))))
    (:NewEnumerator5
      ;[1 0.2036 0 0.5] Create Login Widget
      (bind _errorwgt (Variables|Default|GetErrorWgt)
        (:then
          _)
        (:else
          (bind _returnvalue_8 (UserInterface|CreateWidget "/Game/Widget/HataWg.HataWg_C" _returnvalue_3))
          (Variables|Default|SetErrorWgt _returnvalue_8)))
      (if true
        (UserInterface|Viewport|AddtoViewport _errorwgt 1)
        (Input|SetInputModeUIOnly _returnvalue_3 _errorwgt "DoNotLock")
        (Variables|/Script/Engine.PlayerController|SetbShowMouseCursor _returnvalue_3 true)
        (else
          (Widget|RemovefromParent _errorwgt))))))