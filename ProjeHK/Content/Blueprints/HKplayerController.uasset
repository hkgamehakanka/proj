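; HKgame player controller that holds the player's profile (score, lives, rank, level) and drives lobby music.
; BeginPlay restores the profile from a SaveGame slot or builds a default, and stat updates write it back.
; Music events cycle YouTube embed URLs into the lobby widget's browser.
; Registration, login, player-info and ad events target PHP endpoints with capped retries, but their request helpers are stubbed to return empty strings.
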(event Custom|Playmzk
  (bind _lobywgt (Variables|/Game/Blueprints/HKgameInst.HKgameInst_C|GetLobyWgt (CallFunction|HkgameInst))
    (:then
      (Default|LobiMsc _lobywgt (Variables|Default|GetMuzikUrl))
      (Variables|/Game/Widget/LobiWgt.LobiWgt_C|SetmzkName _lobywgt "Mzk Kapa"))
    (:else)))

(event Custom|RegistryHKgame
  (params (UserName :type String) (Parola :type String) (Mail :type String))
  ;[0 0.5274 0.6771 0.133] Registery işlemler
  (bind _responsecontent (Utilities|DataUpHKgameLoad "Ukomut" "Regstry" "Uid" (Variables|Default|GetHKPlayerName) "Uname" UserName "hkgamehakanka.dx.am/HexFall/LoginRegistry.php" "Upass" Parola "Umail" Mail false :!label _label)
    (:HakanKa
      (if (not (Utilities|Enum|Equal(Enum) _responsecontent "HKgame Kayit Tamam"))
        (if (Utilities|Enum|Equal(Enum) _responsecontent "")
          (Utilities|FlowControl|Delay 1.0)
          (bind _counter (Utilities|FlowControl|DoN 3)
            (:Exit
              (if (not (== _counter 3))
                (goto _label)))))))))

(event Custom|PrvMsc
  (Variables|Default|SetMzkCurt (- (Variables|Default|GetMzkCurt) 1))
  (if (<= (Variables|Default|GetMzkCurt) (Variables|Default|GetMzkPrv))
    (Variables|Default|SetMzkCurt 7))
  (Variables|Default|SetMobil (Utilities|String|Append "www." "youtube.com/embed/"))
  (if (== (Variables|Default|GetMzkCurt) 1)
    (Variables|Default|SetMuzikUrl (Utilities|String|Append (Variables|Default|GetMobil) "Tv6WImqSuxA" "?autoplay=1"))
    (elif (== (Variables|Default|GetMzkCurt) 2)
      (Variables|Default|SetMuzikUrl (Utilities|String|Append (Variables|Default|GetMobil) "UOxkGD8qRB4" "?autoplay=1"))
      (elif (== (Variables|Default|GetMzkCurt) 3)
        (Variables|Default|SetMuzikUrl (Utilities|String|Append (Variables|Default|GetMobil) "O9v6k8sQkcc" "?autoplay=1"))
        (elif (== (Variables|Default|GetMzkCurt) 4)
          (Variables|Default|SetMuzikUrl (Utilities|String|Append (Variables|Default|GetMobil) "ziOYYsU5al4" "?autoplay=1"))
          (elif (== (Variables|Default|GetMzkCurt) 5)
            (Variables|Default|SetMuzikUrl (Utilities|String|Append (Variables|Default|GetMobil) "vojFmQPq87o" "?autoplay=1"))
            (elif (== (Variables|Default|GetMzkCurt) 6)
              (Variables|Default|SetMuzikUrl (Utilities|String|Append (Variables|Default|GetMobil) "RMP6Tip4EwM" "?autoplay=1"))
              (elif (== (Variables|Default|GetMzkCurt) 7)
                (Variables|Default|SetMuzikUrl (Utilities|String|Append (Variables|Default|GetMobil) "WtZbyblyAfw" "?autoplay=1"))
                (else
                  (Variables|Default|SetMuzikUrl (Utilities|String|Append (Variables|Default|GetMobil) "fXGTfD0mt74" "?autoplay=1"))))))))))
  (CallFunction|Playmzk))

(event Custom|LobiDn
  (params (Login :type Boolean)))

(event Custom|GamerPlayerKotrol
  (params (StringUid :type String) (Login :type Boolean))
  (bind _ashkgame_inst (CallFunction|HkgameInst))
  (bind _playerbilgi (Variables|Default|GetPlayerbilgi))
  ;[0 0.5274 0.6771 0.133] HKgame Player controler
  (bind _responsecontent (Utilities|Data2HKgameLoad "hkgamehakanka" "OyunOyunuyozKanka" "Uid" StringUid "hakanka.wartwos2.dx.am/HorseSuper/HKgameLogin.php" :!label _label)
    (:HakanKa
      (if (Utilities|Enum|Equal(Enum) _responsecontent "")
        (Utilities|FlowControl|Delay 1.0)
        (bind _counter (Utilities|FlowControl|DoN 3)
          (:Exit
            (if (not (== _counter 3))
              (goto _label))))
        (else
          (bind _array_element (Utilities|Array|ForEachLoopwithBreak (Utilities|String|ParseIntoArray _responsecontent "|"))
            (:LoopBody
              (Utilities|Array|Add (Variables|Default|GetPlayerbilgi) _array_element))
            (:Completed
              (Variables|Default|SetinfoPlayer (Utilities|Struct|MakePlayerBilgisi (Math|Conversions|ToInteger(Byte) (Utilities|Array|Get(acopy) _playerbilgi)) (Variables|Default|GetHKPlayerName) (Utilities|Array|Get(acopy) _playerbilgi 1) (Utilities|Array|Get(acopy) _playerbilgi 2) "Oyunda" (Utilities|Array|Get(acopy) _playerbilgi 9) (Utilities|Enum|Equal(Enum) (Utilities|Array|Get(acopy) _playerbilgi 3) "1") (Utilities|Enum|Equal(Enum) (Utilities|Array|Get(acopy) _playerbilgi 10) "1") (Math|Conversions|ToInteger(Byte) (Utilities|Array|Get(acopy) _playerbilgi 6)) (Math|Conversions|ToInteger(Byte) (Utilities|Array|Get(acopy) _playerbilgi 5)) (Math|Conversions|ToInteger(Byte) (Utilities|Array|Get(acopy) _playerbilgi 8)) (Math|Conversions|ToInteger(Byte) (Utilities|Array|Get(acopy) _playerbilgi 7)) (Utilities|Enum|Equal(Enum) (Utilities|Array|Get(acopy) _playerbilgi 4) "1")))
              (if (>= (.idVertigo (Utilities|Struct|BreakPlayerBilgisi (Variables|Default|GetinfoPlayer))) 1)
                (Variables|Default|SetOyuncuVar true)
                (if (not (Variables|Default|GetokePlayerRE))
                  (Variables|Default|SetSkopEvent (Utilities|Struct|MakeSkorStrct 0 0 (.Puan (Utilities|Struct|BreakPlayerBilgisi (Variables|Default|GetinfoPlayer))) (.Seviye (Utilities|Struct|BreakPlayerBilgisi (Variables|Default|GetinfoPlayer))) (.Can (Utilities|Struct|BreakPlayerBilgisi (Variables|Default|GetinfoPlayer))) (.Rank (Utilities|Struct|BreakPlayerBilgisi (Variables|Default|GetinfoPlayer)))))
                  ;;[0 0.5274 0.6771 0.133] lobi
                  (if Login
                    (if (.Onay (Utilities|Struct|BreakPlayerBilgisi (Variables|Default|GetinfoPlayer)))
                      (if (.Admin (Utilities|Struct|BreakPlayerBilgisi (Variables|Default|GetinfoPlayer)))
                        (Variables|Default|SetLobiUrl "http://hkgamehakanka.dx.am/HexFall/Reklamlar.php?AdminPanel")
                        (else
                          (Variables|Default|SetLobiUrl "hkgamehakanka.dx.am/HexFall/Avatar.php")))
                      (else
                        (Variables|Default|SetLobiUrl "http://hkgamehakanka.dx.am/HexFall/Reklamlar.php?HexFall")))
                    (Default|MainMenu _ashkgame_inst "NewEnumerator1" false)
                    (Default|MainMenu _ashkgame_inst "NewEnumerator2" true)))
                (else
                  (Variables|Default|SetOyuncuVar false))))))))))

(event Custom|HKgameLogin
  (params (StringValue :type String) (StringPass :type String))
  ;[0 0.5274 0.6771 0.133] Login işlemleri
  (Variables|Default|SetOyuncuName StringValue)
  (bind _responsecontent (Utilities|DataUpHKgameLoad "Ukomut" "Loginn" "Uid" (Variables|Default|GetHKPlayerName) "Uname" StringValue "hkgamehakanka.dx.am/HexFall/LoginRegistry.php" "Upass" StringPass "" "" false :!label _label)
    (:HakanKa
      (if (Utilities|Enum|Equal(Enum) _responsecontent "")
        (Utilities|FlowControl|Delay 1.0)
        (bind _counter (Utilities|FlowControl|DoN 3)
          (:Exit
            (if (not (== _counter 3))
              (goto _label))))
        (elif (Utilities|Enum|Equal(Enum) _responsecontent "HKgame Login Tamam")
          _)))))

(event Custom|SkorHamleTimeEvent
  (params (openEvent :type Integer) (SonTime :type Integer) (SonSkorText :type Integer) (Seviye :type Integer) (Can :type Integer) (Rank :type Integer))
  (Variables|Default|SetOpenEvent (Utilities|Struct|MakeSkorStrct openEvent SonTime SonSkorText Seviye Can Rank)))

(event Custom|MzkKapa
  (bind _lobywgt (Variables|/Game/Blueprints/HKgameInst.HKgameInst_C|GetLobyWgt (CallFunction|HkgameInst))
    (:then
      (Default|LobiMsc _lobywgt "www.google.com")
      (Variables|/Game/Widget/LobiWgt.LobiWgt_C|SetmzkName _lobywgt "Mzk Aç"))
    (:else)))

(event Custom|TglLobiMzk
  (if (Variables|Default|GetTogleMzk)
    (Variables|Default|SetTogleMzk false)
    (CallFunction|MzkKapa)
    (else
      (Variables|Default|SetTogleMzk true)
      (CallFunction|Playmzk))))

(event Custom|HKplayerUserinfoVer
  (params (StringRank :type String) (StringSev :type String) (StringCan :type String) (StringPuan :type String))
  (Variables|Default|SetokePlayerRE true)
  (bind _structout (Utilities|Struct|SetmembersinPlayerBilgisi (Variables|Default|GetinfoPlayer) (Math|Conversions|ToInteger(Byte) StringPuan) (Math|Conversions|ToInteger(Byte) StringCan) (Math|Conversions|ToInteger(Byte) StringRank) (Math|Conversions|ToInteger(Byte) StringSev)))
  (bind _output_get (Variables|Default|SetinfoPlayer _structout))
  (CallFunction|HKsaveData _output_get))

(event Custom|ReklamAlinfo
  ;[0 0.5274 0.6771 0.133] Reklam Event HKgame Online
  (bind _responsecontent (Utilities|Data2HKgameLoad "bak" "info" "sor" "1" "hkgamehakanka.dx.am/HexFall/Reklamlar.php" :!label _label)
    (:HakanKa
      (if (Utilities|Enum|Equal(Enum) _responsecontent "")
        (Utilities|FlowControl|Delay 1.0)
        (bind _counter (Utilities|FlowControl|DoN 3)
          (:Exit
            (if (not (== _counter 3))
              (goto _label))))
        (else
          (CallFunction|ReklamFunSave)
          (Variables|Default|SetUrlTamam true))))))

(event Custom|NextMuzk
  (Variables|Default|SetMzkCurt (+ (Variables|Default|GetMzkCurt) 1))
  (if (>= (Variables|Default|GetMzkCurt) (Variables|Default|GetMzkNext))
    (Variables|Default|SetMzkCurt 0))
  (Variables|Default|SetMobil (Utilities|String|Append "www." "youtube.com/embed/"))
  (if (== (Variables|Default|GetMzkCurt) 1)
    (Variables|Default|SetMuzikUrl (Utilities|String|Append (Variables|Default|GetMobil) "Tv6WImqSuxA" "?autoplay=1"))
    (elif (== (Variables|Default|GetMzkCurt) 2)
      (Variables|Default|SetMuzikUrl (Utilities|String|Append (Variables|Default|GetMobil) "UOxkGD8qRB4" "?autoplay=1"))
      (elif (== (Variables|Default|GetMzkCurt) 3)
        (Variables|Default|SetMuzikUrl (Utilities|String|Append (Variables|Default|GetMobil) "O9v6k8sQkcc" "?autoplay=1"))
        (elif (== (Variables|Default|GetMzkCurt) 4)
          (Variables|Default|SetMuzikUrl (Utilities|String|Append (Variables|Default|GetMobil) "ziOYYsU5al4" "?autoplay=1"))
          (elif (== (Variables|Default|GetMzkCurt) 5)
            (Variables|Default|SetMuzikUrl (Utilities|String|Append (Variables|Default|GetMobil) "vojFmQPq87o" "?autoplay=1"))
            (elif (== (Variables|Default|GetMzkCurt) 6)
              (Variables|Default|SetMuzikUrl (Utilities|String|Append (Variables|Default|GetMobil) "RMP6Tip4EwM" "?autoplay=1"))
              (elif (== (Variables|Default|GetMzkCurt) 7)
                (Variables|Default|SetMuzikUrl (Utilities|String|Append (Variables|Default|GetMobil) "WtZbyblyAfw" "?autoplay=1"))
                (else
                  (Variables|Default|SetMuzikUrl (Utilities|String|Append (Variables|Default|GetMobil) "fXGTfD0mt74" "?autoplay=1"))))))))))
  (CallFunction|Playmzk))

(event EventBeginPlay
  (bind (_output _returnvalue) (CallFunction|HKgameData))
  (bind (_hatirla _vertigodata) (CallFunction|HKloadData))
  (if _hatirla
    (Variables|Default|SetinfoPlayer _vertigodata)
    (else
      (Variables|Default|SetinfoPlayer (Utilities|Struct|MakePlayerBilgisi 0 _output "WestHaan" "HKgame.yt@gmail.com" "Oyunda" _returnvalue)))))

(event EventTick
  (params (DeltaSeconds :type Float%20%28single-precision%29)))

(fn ConstructionScript)

(fn HKloadLogin
  (params (SlotName :type String)))

(fn HKsaveLogin
  (params (SlotName :type String) (Hatirla :type Boolean) (VertigoName :type String) (VertigoParola :type String) (VertigoID :type String)))

(fn ReklamFunSave
  (params (Option%201 :type String) (Option%202 :type String) (Option%203 :type String) (Option%204 :type String) (Option%205 :type String) (Rek1 :type String) (Rek2 :type String) (Rek3 :type String))
  (Variables|Default|SetRek1 Option%201)
  (Variables|Default|SetRek2 Option%202)
  (Variables|Default|SetRek3 Option%203)
  (Variables|Default|SetRek4 Option%204)
  (Variables|Default|SetRek5 Option%205)
  (Variables|Default|SetUrlRek1 Rek1)
  (Variables|Default|SetUrlRek2 Rek2)
  (Variables|Default|SetUrlRek3 Rek3))

(fn RekFunLoad
  (return (Variables|Default|GetRek1) (Variables|Default|GetRek2) (Variables|Default|GetRek3) (Variables|Default|GetRek4) (Variables|Default|GetRek5) (Variables|Default|GetUrlRek1) (Variables|Default|GetUrlRek2) (Variables|Default|GetUrlRek3)))

(fn HkgameInst
  (bind _ashkgame_inst (Utilities|Casting|CastToHKgameInst (Game|GetGameInstance)))
  (return _ashkgame_inst))

(fn HKloadData
  (bind _hkgameslotvertigo (Variables|Default|GetHKgameSlotVertigo))
  (bind _returnvalue (SaveGame|DoesSaveGameExist _hkgameslotvertigo))
  (if _returnvalue
    (bind _returnvalue_2 (SaveGame|LoadGamefromSlot _hkgameslotvertigo))
    (bind _asvertigo_hkgame_save (Utilities|Casting|CastToVertigoHKgameSave _returnvalue_2))
    (bind (_hatirla _vertigodata) (Default|LoadVertigoData _asvertigo_hkgame_save))
    (return _hatirla _vertigodata)
    (else
      (return false ""))))

(fn HKsaveData
  (params (VertigoData :type Player%20Bilgisi%20Structure))
  (Variables|Default|GetVertigoHKgameSave
    (:then
      _)
    (:else
      (bind _returnvalue (SaveGame|CreateSaveGameObject "/Game/Blueprints/VertigoHKgameSave.VertigoHKgameSave_C"))
      (Variables|Default|SetVertigoHKgameSave _returnvalue)))
  (Default|SaveVertigoData (Variables|Default|GetVertigoHKgameSave) true VertigoData)
  (bind _returnvalue_2 (SaveGame|SaveGametoSlot (Variables|Default|GetVertigoHKgameSave) (Variables|Default|GetHKgameSlotVertigo)))
  (return _returnvalue_2))

(fn HKgameData
  (bind _returnvalue (Math|DateTime|Now))
  (bind (_year _month _day _hour _minute) (Math|DateTime|BreakDateTime _returnvalue))
  (return (Utilities|Array|Get(acopy) (Utilities|String|ParseIntoArray (PlayerState|GetPlayerName (Variables|GetPlayerState)) "-")) (Utilities|String|Append (Utilities|String|ToString(Integer) _year) "/" (Utilities|String|ToString(Integer) _month) "/" (Utilities|String|ToString(Integer) _day) "(" (Utilities|String|ToString(Integer) _hour) ":" (Utilities|String|ToString(Integer) _minute) ")")))